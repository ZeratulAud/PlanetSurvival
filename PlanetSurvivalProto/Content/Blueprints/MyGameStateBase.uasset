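; Game state Blueprint that sets up the game's item inventory records for fruit, stem fibers, a fruit plant sample and a lore note.
; On BeginPlay, a Sequence adds one MyItem per type, gives it an enum name and zero amount, and prints that name.
; The final step collects all four items into the AllItems array.
; The UpdateInventory event is an empty stub.
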(event Custom|UpdateInventory)

(event EventBeginPlay
  (bind _all_items (Variables|Default|GetAll_Items))
  (Utilities|FlowControl|Sequence
    (:then_0
      (bind _returnvalue (AddComponent|AddMyItem))
      (bind _output_get (Variables|Default|SetFruit _returnvalue))
      (bind _output_get_2 (Variables|/Game/Inventory/MyItem.MyItem_C|SetName _output_get "NewEnumerator0"))
      (Variables|/Game/Inventory/MyItem.MyItem_C|SetAmount _output_get 0)
      (Development|PrintString (Utilities|String|EnumtoString _output_get_2)))
    (:then_1
      (bind _returnvalue_2 (AddComponent|AddMyItem))
      (bind _output_get_3 (Variables|Default|SetStemFibers _returnvalue_2))
      (bind _output_get_4 (Variables|/Game/Inventory/MyItem.MyItem_C|SetName _output_get_3 "NewEnumerator1"))
      (Variables|/Game/Inventory/MyItem.MyItem_C|SetAmount _output_get_3 0)
      (Development|PrintString (Utilities|String|EnumtoString _output_get_4)))
    (:then_2
      (bind _returnvalue_3 (AddComponent|AddMyItem))
      (bind _output_get_5 (Variables|Default|SetFruitPlantSample _returnvalue_3))
      (bind _output_get_6 (Variables|/Game/Inventory/MyItem.MyItem_C|SetName _output_get_5 "NewEnumerator2"))
      (Variables|/Game/Inventory/MyItem.MyItem_C|SetAmount _output_get_5 0)
      (Development|PrintString (Utilities|String|EnumtoString _output_get_6)))
    (:then_3
      (bind _returnvalue_4 (AddComponent|AddMyItem))
      (bind _output_get_7 (Variables|Default|SetLoreNote#1 _returnvalue_4))
      (bind _output_get_8 (Variables|/Game/Inventory/MyItem.MyItem_C|SetName _output_get_7 "NewEnumerator3"))
      (Variables|/Game/Inventory/MyItem.MyItem_C|SetAmount _output_get_7 0)
      (Development|PrintString (Utilities|String|EnumtoString _output_get_8)))
    (:then_4
      (Utilities|Array|Add _all_items (Variables|Default|GetFruit))
      (Utilities|Array|Add _all_items (Variables|Default|GetStemFibers))
      (Utilities|Array|Add _all_items (Variables|Default|GetFruitPlantSample))
      (Utilities|Array|Add _all_items (Variables|Default|GetLoreNote#1)))))

(event EventTick
  (params (DeltaSeconds :type Float%20%28single-precision%29)))

(fn ConstructionScript)